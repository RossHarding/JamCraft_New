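; Allomantic beam effect actor that draws a particle beam between the player's view and a referenced metal object.
; A gate opened at BeginPlay lets Tick set the beam's source just below the camera and its target at the metal's mesh location.
; Each update also sets a fixed initial beam size and shows the beam only while the player's pawn is within range of the metal.
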(event `self.ReceiveTick`
  (params (DeltaSeconds :type "Float (single-precision)"))
  (bind _allomanticbeamparticlesystem (`self.AllomanticBeamParticleSystem`))
  (bind (_returnvalue_x _returnvalue_y _returnvalue_z) (`KismetMathLibrary.BreakVector` (`PlayerCameraManager.GetCameraLocation` (`PlayerController.PlayerCameraManager` (`GameplayStatics.GetPlayerController` 0)))))
  ;[1 1 1] Comment
  (`/Engine/EditorBlueprintResources/StandardMacros.Gate` true :!label _label
    (:`Exit`
      (`SceneComponent.SetVisibility` _allomanticbeamparticlesystem (< (`self.GetDistanceTo` (`Controller.K2_GetPawn` (`GameplayStatics.GetPlayerController` 0)) (`self.MetalRef`)) 2000.0) false)
      (`ParticleSystemComponent.SetVectorParameter` _allomanticbeamparticlesystem "InitialSize" (0.2 0.0 0.0))
      (`ParticleSystemComponent.SetBeamTargetPoint` _allomanticbeamparticlesystem 0 (`SceneComponent.K2_GetComponentLocation` (`/Game/FX/AllomanticParticleBP.StaticMesh1` (`self.MetalRef`))) 0)
      (`ParticleSystemComponent.SetBeamSourcePoint` _allomanticbeamparticlesystem 0 (`KismetMathLibrary.MakeVector` _returnvalue_x _returnvalue_y (+ _returnvalue_z -5.0)) 0))))

(event `self.ReceiveBeginPlay`
  ;[1 1 1] Comment
  (goto _label :!via `Open`))

(event `self.ReceiveDestroyed`
  ;[1 1 1] Comment
  (cast `` (`GameplayStatics.GetPlayerCharacter` 0)))

(fn `UserConstructionScript`)