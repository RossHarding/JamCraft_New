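; ElectricArc_BP is an effect actor that draws an electric arc beam from the player's right hand to their laser hit location.
; BeginPlay caches the player's AlphoCharacter_BP and opens a gate that lets Tick through.
; Each tick sets the beam particle system's initial size, targets the character's LaserHitLocation, and sources the beam at the mesh's hand_r socket.
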(event `self.ReceiveTick`
  (params (DeltaSeconds :type "Float (single-precision)"))
  ;[1 1 1] Comment
  (`/Engine/EditorBlueprintResources/StandardMacros.Gate` true :!label _label
    (:`Exit`
      (`ParticleSystemComponent.SetVectorParameter` (`self.AllomanticBeamParticleSystem`) "InitialSize" (2.0 2.0 2.0))
      (`ParticleSystemComponent.SetBeamTargetPoint` (`self.AllomanticBeamParticleSystem`) 0 (`/Game/Character/AlphoCharacter_BP.LaserHitLocation` (`self.Char_ref`)) 0)
      (`ParticleSystemComponent.SetBeamSourcePoint` (`self.AllomanticBeamParticleSystem`) 0 (`SceneComponent.GetSocketLocation` (`Character.Mesh` (`self.Char_ref`)) "hand_r") 0))))

(event `self.ReceiveBeginPlay`
  ;[1 1 1] Comment
  (bind _asalpho_character_bp (cast `/Game/Character/AlphoCharacter_BP` (`GameplayStatics.GetPlayerCharacter` 0)))
  (set `self.Char_ref` _asalpho_character_bp)
  (goto _label :!via `Open`))

(event `self.ReceiveDestroyed`
  ;[1 1 1] Comment
)

(fn `UserConstructionScript`)