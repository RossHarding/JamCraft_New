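; Laser beam effect actor that draws four particle beams from the player character's right hand to its laser hit location.
; BeginPlay caches the AlphoCharacter_BP player reference, prints a debug string and opens a gate for Tick.
; Each tick resets the beams' InitialSize parameter and moves their source and target points, offsetting them along the character's up and right vectors to form a diamond-shaped bundle.
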(event `self.ReceiveTick`
  (params (DeltaSeconds :type "Float (single-precision)"))
  (bind _char_ref (`self.Char_ref`))
  (bind _char_ref_2 (`self.Char_ref`))
  (bind _char_ref_3 (`self.Char_ref`))
  (bind _returnvalue (`self.GetActorRightVector` _char_ref_3))
  (bind _returnvalue_2 (`self.GetActorRightVector` _char_ref_2))
  (bind _laserhitlocation (`/Game/Character/AlphoCharacter_BP.LaserHitLocation` _char_ref_2))
  (bind _returnvalue_3 (`SceneComponent.GetSocketLocation` (`Character.Mesh` _char_ref) "hand_r"))
  ;[1 1 1] Comment
  (`/Engine/EditorBlueprintResources/StandardMacros.Gate` true :!label _label
    (:`Exit`
      (`ParticleSystemComponent.SetVectorParameter` (`self.AllomanticBeamParticleSystem`) "InitialSize" (2.0 2.0 2.0))
      (`ParticleSystemComponent.SetVectorParameter` (`self.ParticleSystem`) "InitialSize" (2.0 2.0 2.0))
      (`ParticleSystemComponent.SetVectorParameter` (`self.ParticleSystem1`) "InitialSize" (2.0 2.0 2.0))
      (`ParticleSystemComponent.SetVectorParameter` (`self.ParticleSystem2`) "InitialSize" (2.0 2.0 2.0))
      (`ParticleSystemComponent.SetBeamTargetPoint` (`self.AllomanticBeamParticleSystem`) 0 (+ (* (`self.GetActorUpVector` _char_ref_2) 2.0) _laserhitlocation) 0)
      (`ParticleSystemComponent.SetBeamTargetPoint` (`self.ParticleSystem`) 0 (+ _laserhitlocation (* _returnvalue_2 2.5)) 0)
      (`ParticleSystemComponent.SetBeamTargetPoint` (`self.ParticleSystem1`) 0 (+ _laserhitlocation (* _returnvalue_2 -2.5)) 0)
      (`ParticleSystemComponent.SetBeamTargetPoint` (`self.ParticleSystem2`) 0 (+ _laserhitlocation (* (`self.GetActorUpVector` _char_ref_2) -2.0)) 0)
      (`ParticleSystemComponent.SetBeamSourcePoint` (`self.AllomanticBeamParticleSystem`) 0 (+ (* (`self.GetActorUpVector` _char_ref) 2.0) _returnvalue_3) 0)
      (`ParticleSystemComponent.SetBeamSourcePoint` (`self.ParticleSystem`) 0 (+ _returnvalue_3 (* _returnvalue 2.5)) 0)
      (`ParticleSystemComponent.SetBeamSourcePoint` (`self.ParticleSystem1`) 0 (+ _returnvalue_3 (* _returnvalue -2.5)) 0)
      (`ParticleSystemComponent.SetBeamSourcePoint` (`self.ParticleSystem2`) 0 (+ _returnvalue_3 (* (`self.GetActorUpVector` _char_ref_3) -2.0)) 0))))

(event `self.ReceiveBeginPlay`
  ;[1 1 1] Comment
  (bind _asalpho_character_bp (cast `/Game/Character/AlphoCharacter_BP` (`GameplayStatics.GetPlayerCharacter` 0)))
  (set `self.Char_ref` _asalpho_character_bp)
  (`KismetSystemLibrary.PrintString` "3245135")
  (goto _label :!via `Open`))

(event `self.ReceiveDestroyed`
  ;[1 1 1] Comment
)

(fn `UserConstructionScript`)